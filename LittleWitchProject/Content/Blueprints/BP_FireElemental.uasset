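; BP_FireElemental is an enemy that shoots fireballs when it sees the side-scroller player character.
; PawnSensing triggers a BP_EnemyFireball spawn at ProjectileSpawnLocation, launched by an impulse along the mesh's forward vector.
; A boolean gate and short delay act as the firing cooldown.
; Logic to rotate the spawn point toward the player exists but is disconnected, so shots are not aimed.
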(event OnSeePawn(PawnSensing)
  (params (Pawn :type Pawn%20Object%20Reference))
  (bind _asside_scroller_character (Utilities|Casting|CastToSideScrollerCharacter Pawn))
  (Utilities|FlowControl|Sequence
    (:then_1
      (if (Variables|Default|GetSpawnProjectile)
        (bind _returnvalue (Game|SpawnActorfromClass "/Game/Blueprints/BP_EnemyFireball.BP_EnemyFireball_C" (Transformation|GetWorldTransform (Variables|Default|GetProjectileSpawnLocation)) "AlwaysSpawn" 0 0))
        (Physics|AddImpulse (Variables|/Game/Blueprints/BP_EnemyFireball.BP_EnemyFireball_C|GetSphere _returnvalue) (* (Math|Vector|GetForwardVector (Variables|Character|GetMesh)) (Variables|Default|GetShootAmount)) "None" true)
        (Variables|Default|SetSpawnProjectile false)
        (Utilities|FlowControl|Delay 1.9)
        (Variables|Default|SetSpawnProjectile true)))))

(event EventBeginPlay)

(event Collision|EventActorBeginOverlap
  (params (OtherActor :type Actor%20Object%20Reference)))

(event EventTick
  (params (DeltaSeconds :type Float%20%28single-precision%29)))

(fn ConstructionScript)